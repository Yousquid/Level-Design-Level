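; Enemy that roams the navmesh, chases pawns it sees, and opens FirstPersonMap when it hits the first-person player character.
; AIMoveTo chains random destinations while wandering and targets the pawn spotted by PawnSensing.
; A DoOnce gates the switch to run animation and speed.
; A retriggerable delay, refreshed by sightings, restores walking, resets that gate and resumes wandering.
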(event OnSeePawn(PawnSensing)
  (params (Pawn :type Pawn%20Object%20Reference))
  (Utilities|FlowControl|Sequence
    (:then_0
      (Utilities|FlowControl|DoOnce false
        (:Completed
          (Components|Animation|PlayAnimation (Variables|Character|GetMesh) "/Game/Characters/Mannequins/Animations/Quinn/MF_Run_Fwd.MF_Run_Fwd" true)
          (Variables|/Script/Engine.CharacterMovementComponent|SetMaxWalkSpeed (Variables|Character|GetCharacterMovement) 715.0))))
    (:then_1
      (AI|AIMoveTo self "0, 0, 0" Pawn 5.0 false
        (:then
          (Utilities|FlowControl|RetriggerableDelay 2.0)
          (Components|Animation|PlayAnimation (Variables|Character|GetMesh) "/Game/Characters/Mannequins/Animations/Manny/MM_Walk_Fwd.MM_Walk_Fwd" true)
          (Variables|/Script/Engine.CharacterMovementComponent|SetMaxWalkSpeed (Variables|Character|GetCharacterMovement) 3e+02)
          (CallFunction|CanSprintAgain)
          (CallFunction|MovetoRandomLocation))))))

(event Custom|MoveToRandomLocation
  (bind _randomlocation (Class|NavigationSystemV1|GetRandomLocationinNavigableRadius (Transformation|GetActorLocation) 4e+03 0 0))
  (AI|AIMoveTo self _randomlocation 0 5.0 false
    (:OnSuccess
      (CallFunction|MovetoRandomLocation))))

(event Custom|CanSprintAgain
  (Utilities|FlowControl|DoOnce false) ; enters at Reset
)

(event EventBeginPlay
  (CallFunction|MovetoRandomLocation))

(event Collision|EventHit
  (params (MyComp :type Primitive%20Component%20Object%20Reference) (Other :type Actor%20Object%20Reference) (OtherComp :type Primitive%20Component%20Object%20Reference) (bSelfMoved :type Boolean) (HitLocation :type Vector :default "0, 0, 0") (HitNormal :type Vector :default "0, 0, 0") (NormalImpulse :type Vector :default "0, 0, 0") (Hit :type Hit%20Result%20Structure%20%28by%20ref%29))
  (Utilities|Casting|CastToBP_FirstPersonCharacter Other)
  (Game|OpenLevel(byName) "FirstPersonMap"))

(fn ConstructionScript)